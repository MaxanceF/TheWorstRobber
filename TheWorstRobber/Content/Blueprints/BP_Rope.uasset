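; Climbable rope actor that the third-person player attaches to or releases with E.
; Attaching pins the cable end to the player and physics-constrains their simulated capsule to the rope's cube, with character movement disabled.
; Climb events nudge the constraint's Z limit and reference, then update cable length and bottom collision box; only climbing up has a height check.
; Detaching restores falling and, after a delay, stops capsule physics unless reattached.
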(event `E Pressed`
  ; When E is pressed, attach or detach rope for player
  (if (`/Game/Blueprints/BP_ThirdPersonCharacter.IsPlayerAttached` (`self.Player`))
    (`self.DetachRopeToPlayer`)
    (else
      (`self.AttachRopeToPlayer`))))

(event `Climb Down The Rope`
  (bind (_returnvalue_x _returnvalue_y _returnvalue_z) (`KismetMathLibrary.BreakVector` (`self.K2_GetActorLocation`)))
  (bind _physicsconstraint (`self.PhysicsConstraint`))
  (bind (_returnvalue_x_2 _returnvalue_y_2 _returnvalue_z_2) (`KismetMathLibrary.BreakVector` (`self.K2_GetActorLocation` (`self.Player`))))
  (bind _returnvalue (+ (`self.Ref Position Z`) 0.5))
  (bind _returnvalue_2 (+ (`self.Limit Size`) 0.1))
  (bind _returnvalue_3 (- _returnvalue_z _returnvalue_z_2))
  ; Climb Down Event on Rope
  (if (`/Game/Blueprints/BP_ThirdPersonCharacter.IsPlayerAttached` (`self.Player`))
    (if true
      (`PhysicsConstraintComponent.SetLinearZLimit` _physicsconstraint "LCM_Limited" _returnvalue_2)
      (set `self.Limit Size` _returnvalue_2)
      (`PhysicsConstraintComponent.SetConstraintReferencePosition` _physicsconstraint "Frame2" (`KismetMathLibrary.MakeVector` 0.0 0.0 _returnvalue))
      (set `self.Ref Position Z` _returnvalue)
      (set `CableComponent.CableLength` _returnvalue_3 (`self.Cable`))
      (`SceneComponent.K2_SetRelativeLocation` (`self.BottomRopeBoxCollision`) (`KismetMathLibrary.MakeVector` 0.0 0.0 (* _returnvalue_3 -3.0)) false false))))

(event `Climb Up The Rope`
  (bind (_returnvalue_x _returnvalue_y _returnvalue_z) (`KismetMathLibrary.BreakVector` (`self.K2_GetActorLocation`)))
  (bind _physicsconstraint (`self.PhysicsConstraint`))
  (bind (_returnvalue_x_2 _returnvalue_y_2 _returnvalue_z_2) (`KismetMathLibrary.BreakVector` (`SceneComponent.K2_GetComponentLocation` (`self.ClimbUpArrowRef`))))
  (bind (_returnvalue_x_3 _returnvalue_y_3 _returnvalue_z_3) (`KismetMathLibrary.BreakVector` (`self.K2_GetActorLocation` (`GameplayStatics.GetPlayerCharacter` 0))))
  (bind (_returnvalue_x_4 _returnvalue_y_4 _returnvalue_z_4) (`KismetMathLibrary.BreakVector` (`self.K2_GetActorLocation` (`self.Player`))))
  (bind _returnvalue (- (`self.Limit Size`) 0.1))
  (bind _returnvalue_2 (- (`self.Ref Position Z`) 0.5))
  (bind _returnvalue_3 (- _returnvalue_z _returnvalue_z_4))
  ; Climb up Event on Rope
  (if (`/Game/Blueprints/BP_ThirdPersonCharacter.IsPlayerAttached` (`self.Player`))
    (if (>= _returnvalue_z_2 _returnvalue_z_3)
      (`PhysicsConstraintComponent.SetLinearZLimit` _physicsconstraint "LCM_Limited" _returnvalue)
      (set `self.Limit Size` _returnvalue)
      (`PhysicsConstraintComponent.SetConstraintReferencePosition` _physicsconstraint "Frame2" (`KismetMathLibrary.MakeVector` 0.0 0.0 _returnvalue_2))
      (set `self.Ref Position Z` _returnvalue_2)
      (set `CableComponent.CableLength` _returnvalue_3 (`self.Cable`))
      (`SceneComponent.K2_SetRelativeLocation` (`self.BottomRopeBoxCollision`) (`KismetMathLibrary.MakeVector` 0.0 0.0 (* _returnvalue_3 -3.0)) false false))))

(event `self.ReceiveBeginPlay`
  ; GetPlayerPawn at BeginPlay
  (bind _asbp_third_person_character (cast `/Game/Blueprints/BP_ThirdPersonCharacter` (`GameplayStatics.GetPlayerPawn` 0)))
  (set `self.Player` _asbp_third_person_character))

(fn `UserConstructionScript`)